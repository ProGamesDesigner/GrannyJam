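; BP_Door is an interactable door that moves the player to another level.
; Player overlap caches the BP_GameInstance reference, which Interact uses to store the door's TransitionName so it persists across the level change.
; Interact then shows the WB_LoadScreen widget and starts a one-second timer that calls LevelTransition to open the level named by LevelName.
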(event EventBeginPlay
  (bind _asbp_first_person_character (Utilities|Casting|CastToBP_FirstPersonCharacter (Game|GetPlayerCharacter 0)))
  (Variables|Default|SetAs%20BP%20First%20Person%20Character _asbp_first_person_character))

(event Collision|EventActorBeginOverlap
  (params (OtherActor :type Actor%20Object%20Reference))
  (if (== OtherActor (Game|GetPlayerCharacter 0))
    (bind _asbp_game_instance (Utilities|Casting|CastToBP_GameInstance (Game|GetGameInstance)))))

(event Collision|EventActorEndOverlap
  (params (OtherActor :type Actor%20Object%20Reference))
  (if (== OtherActor (Game|GetPlayerCharacter 0))
    _))

(event EventInteract
  (Variables|/Game/Blueprints/BP_GameInstance.BP_GameInstance_C|SetTransitionName (stale Collision|EventActorBeginOverlap _asbp_game_instance) (Variables|Default|GetTransitionName))
  (bind _returnvalue (UserInterface|CreateWidget "/Game/UI/WB_LoadScreen.WB_LoadScreen_C"))
  (UserInterface|Viewport|AddtoViewport _returnvalue 0)
  (Utilities|Time|SetTimerbyFunctionName 0 "LevelTransition" 1.0))

(fn ConstructionScript)

(fn LevelTransition
  (Game|OpenLevel(byName) (Variables|Default|GetLevel%20Name) false))